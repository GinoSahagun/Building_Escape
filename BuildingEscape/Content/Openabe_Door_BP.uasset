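; Openable door actor that swings open and closed in response to its OpenDoor component's OnOpen and OnClose events.
; The DoorSwing timeline plays forward or reverses, combining its DoorAngle yaw with the rotation cached at BeginPlay so the swing is relative to the placed orientation.
; A timeline event track plays the lock sound at the door's location.
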(event OnClose(OpenDoor)
  (bind _door_angle (Timeline|Door%20Swing Reverse)
    (:Update
      (Transformation|SetActorRotation (Math|Rotator|CombineRotators (Math|Rotator|MakeRotator 0.0 0.0 _door_angle) (Variables|Default|Getinital%20Rotation))))
    (:Sound%20Trigger%20Lock
      (Audio|PlaySoundatLocation "/Game/Audio/door-lock.door-lock" (Transformation|GetActorLocation)))))

(event OnOpen(OpenDoor)
  (bind _door_angle (Timeline|Door%20Swing Play)
    (:Update
      (Transformation|SetActorRotation (Math|Rotator|CombineRotators (Math|Rotator|MakeRotator 0.0 0.0 _door_angle) (Variables|Default|Getinital%20Rotation))))
    (:Sound%20Trigger%20Lock
      (Audio|PlaySoundatLocation "/Game/Audio/door-lock.door-lock" (Transformation|GetActorLocation)))))

(event EventBeginPlay
  (Variables|Default|Setinital%20Rotation (Transformation|GetActorRotation)))

(fn ConstructionScript)